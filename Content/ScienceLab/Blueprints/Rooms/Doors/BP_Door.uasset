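; BP_Door is a sliding lab door, single or double, that opens on overlap and closes when an overlap ends.
; The construction script assigns meshes, and BeginPlay sets opening distance and widens collision for double doors.
; A timeline slides the panels along local Y, mirroring the right one.
; When Fatal is set, only BP_Body opens it, first triggering EOT on that actor's AC_0X00A21E component if present.
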(event OnComponentEndOverlap(Collision)
  (params (OverlappedComponent :type Primitive%20Component%20Object%20Reference) (OtherActor :type Actor%20Object%20Reference) (OtherComp :type Primitive%20Component%20Object%20Reference) (OtherBodyIndex :type Integer))
  ;[1 1 1] DoorOpening
  (bind _newtrack_0 (Timeline|Timeline Reverse)
    (:Update
      (Transformation|SetRelativeLocation (Variables|Default|GetDoorL) (Math|Vector|MakeVector 0.0 (Math|Float|Lerp 0.0 (Variables|Default|GetMaxOpening) _newtrack_0) 0.0) false false)
      (bind _doorr (Variables|Default|GetDoorR)
        (:then
          (Transformation|SetRelativeLocation _doorr (Math|Vector|MakeVector 0.0 (* (Math|Float|Lerp 0.0 (Variables|Default|GetMaxOpening) _newtrack_0) -1.0) 0.0) false false))
        (:else)))))

(event OnComponentBeginOverlap(Collision)
  (params (OverlappedComponent :type Primitive%20Component%20Object%20Reference) (OtherActor :type Actor%20Object%20Reference) (OtherComp :type Primitive%20Component%20Object%20Reference) (OtherBodyIndex :type Integer) (bFromSweep :type Boolean) (SweepResult :type Hit%20Result%20Structure%20%28by%20ref%29))
  ;[1 0 0] FatalCodeDoor42
  (if (Variables|Default|GetFatal?)
    (bind _asbp_body (Utilities|Casting|CastToBP_Body OtherActor))
    (Utilities|FlowControl|Sequence
      (:then_0
        (Utilities|IsValid (Actor|GetComponentbyClass _asbp_body "/Game/ScienceLab/SecuritySystem/AC_0X00A21E.AC_0X00A21E_C")
          (:Is%20Valid
            (Default|EOT (Actor|GetComponentbyClass _asbp_body "/Game/ScienceLab/SecuritySystem/AC_0X00A21E.AC_0X00A21E_C")))))
      (:then_1
        ;[1 1 1] DoorOpening
        (bind _newtrack_0 (Timeline|Timeline Play)
          (:Update
            (Transformation|SetRelativeLocation (Variables|Default|GetDoorL) (Math|Vector|MakeVector 0.0 (Math|Float|Lerp 0.0 (Variables|Default|GetMaxOpening) _newtrack_0) 0.0) false false)
            (bind _doorr (Variables|Default|GetDoorR)
              (:then
                (Transformation|SetRelativeLocation _doorr (Math|Vector|MakeVector 0.0 (* (Math|Float|Lerp 0.0 (Variables|Default|GetMaxOpening) _newtrack_0) -1.0) 0.0) false false))
              (:else))))))
    (else
      (Timeline|Timeline Play))))

(event Collision|EventActorBeginOverlap
  (params (OtherActor :type Actor%20Object%20Reference)))

(event EventTick
  (params (DeltaSeconds :type Float%20%28single-precision%29)))

(event EventBeginPlay
  (bind _collision (Variables|Default|GetCollision))
  (bind _returnvalue (Transformation|GetWorldTransform _collision))
  (if (Variables|Default|GetDouble%20Door?)
    (Variables|Default|SetMaxOpening 6e+01)
    (Transformation|SetWorldTransform _collision (Math|Transform|MakeTransform (.location _returnvalue) (.rotation _returnvalue) (Math|Vector|MakeVector (.x (.scale _returnvalue)) (* (.y (.scale _returnvalue)) 1.75) (.z (.scale _returnvalue)))) false false)))

(fn ConstructionScript
  (if (not (Variables|Default|GetDouble%20Door?))
    (Components|StaticMesh|SetStaticMesh (Variables|Default|GetDoorL) (Variables|Default|GetDoorLeft))
    (Components|StaticMesh|SetStaticMesh (Variables|Default|GetDoorJamb) (Variables|Default|GetDoorJambi))
    (else
      (Components|StaticMesh|SetStaticMesh (Variables|Default|GetDoorL) (Variables|Default|GetDoorLeft))
      (Components|StaticMesh|SetStaticMesh (Variables|Default|GetDoorJamb) (Variables|Default|GetDoorJambi))
      (Components|StaticMesh|SetStaticMesh (Variables|Default|GetDoorR) (Variables|Default|GetDoorRight)))))